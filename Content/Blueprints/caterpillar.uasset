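; Caterpillar enemy for a 2D side-scroller that walks back and forth and damages actors tagged "player" on hit.
; Tick drives movement along X and yaws the sprite to match a direction flag, which capsule hits toggle.
; A Box2 hit from the 2DSideScrollerCharacter shows the death flipbook, then destroys it after a short delay.
; A MoveRight axis handler can also set direction and add movement.
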(event OnComponentHit(Box2)
  (params (HitComponent :type Primitive%20Component%20Object%20Reference) (OtherActor :type Actor%20Object%20Reference) (OtherComp :type Primitive%20Component%20Object%20Reference) (NormalImpulse :type Vector :default "0, 0, 0") (Hit :type Hit%20Result%20Structure%20%28by%20ref%29))
  (Utilities|Casting|CastTo2DSideScrollerCharacter OtherActor)
  (Utilities|FlowControl|Sequence
    (:then_0
      (Variables|Default|SetLSprite "/Game/assets/sprites/death_.death_")
      (Utilities|FlowControl|Delay 0.2)
      (Actor|DestroyActor))
    (:then_1
      (Sprite|SetFlipbook (Variables|Default|GetSprite) (Variables|Default|GetLSprite)))))

(event OnComponentHit(CapsuleComponent)
  (params (HitComponent :type Primitive%20Component%20Object%20Reference) (OtherActor :type Actor%20Object%20Reference) (OtherComp :type Primitive%20Component%20Object%20Reference) (NormalImpulse :type Vector :default "0, 0, 0") (Hit :type Hit%20Result%20Structure%20%28by%20ref%29))
  (Variables|Default|SetbisMovingRight (not (Variables|Default|GetbisMovingRight))))

(event Custom|Direction
  (Transformation|SetRelativeRotation (Variables|Default|GetSprite) (Math|Rotator|MakeRotator 0.0 0.0 (Math|Float|SelectFloat 0.0 1.8e+02 (Variables|Default|GetbisMovingRight))) false false)
  (Pawn|Input|AddMovementInput (Math|Vector|SelectVector "1.000000, 0, 0" "-1.000000, 0, 0" (Variables|Default|GetbisMovingRight)) 1.0 false))

(event Collision|EventHit
  (params (MyComp :type Primitive%20Component%20Object%20Reference) (Other :type Actor%20Object%20Reference) (OtherComp :type Primitive%20Component%20Object%20Reference) (bSelfMoved :type Boolean) (HitLocation :type Vector :default "0, 0, 0") (HitNormal :type Vector :default "0, 0, 0") (NormalImpulse :type Vector :default "0, 0, 0") (Hit :type Hit%20Result%20Structure%20%28by%20ref%29))
  (if (Actor|ActorHasTag Other "player")
    (Utilities|FlowControl|Delay 0.21)
    (Game|Damage|ApplyDamage Other (Variables|Default|Getdmg) 0 0)))

(event EventTick
  (params (DeltaSeconds :type Float%20%28single-precision%29))
  (CallFunction|Direction))

(event Input|AxisEvents|InputAxisMoveRight
  (params (AxisValue :type Float%20%28single-precision%29))
  (Math|Float|CompareFloat AxisValue 0.0
    (:>
      (Variables|Default|SetbisMovingRight true))
    (:<
      (Variables|Default|SetbisMovingRight false)))
  (Pawn|Input|AddMovementInput "1.000000, 0, 0" AxisValue false))

(fn ConstructionScript)