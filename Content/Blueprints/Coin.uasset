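; Coin pickup actor for a 2D side-scroller, built around a Paper2D sprite.
; On any actor overlap it casts player pawn 0 to 2DSideScrollerCharacter, without checking which actor overlapped.
; If the cast succeeds, it plays a coin sound, increments the character's Coins and Score directly, then destroys its sprite and itself.
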(event EventBeginPlay)

(event Collision|EventActorBeginOverlap
  (params (OtherActor :type Actor%20Object%20Reference))
  (bind _as2dside_scroller_character (Utilities|Casting|CastTo2DSideScrollerCharacter (Game|Player|GetPlayerPawn 0)))
  (Audio|PlaySound2D "/Game/assets/Music/coin_ver_2.coin_ver_2" 1.0 1.0 0.0 0 0)
  (Variables|/Game/Blueprints/2DSideScrollerCharacter.2DSideScrollerCharacter_C|SetCoins _as2dside_scroller_character (+ (Variables|/Game/Blueprints/2DSideScrollerCharacter.2DSideScrollerCharacter_C|GetCoins _as2dside_scroller_character) 1))
  (Variables|/Game/Blueprints/2DSideScrollerCharacter.2DSideScrollerCharacter_C|SetScore _as2dside_scroller_character (+ (Variables|/Game/Blueprints/2DSideScrollerCharacter.2DSideScrollerCharacter_C|GetScore _as2dside_scroller_character) 100))
  (Components|DestroyComponent (Variables|Default|GetPaperSprite))
  (Actor|DestroyActor))

(fn ConstructionScript)